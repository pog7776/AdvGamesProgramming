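; Enemy character Blueprint, named for NavMesh and behavior tree movement, that provides Attack and Die events.
; BeginPlay caches its MyAIControllerNM controller.
; Attack stops movement, switches the mesh to single-node animation, then restores the Animation Blueprint after a fixed delay.
; Die runs on authority only, making the same stop and animation switch before destroying the actor immediately, with no delay.
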(event EventBeginPlay
  (bind _asmy_aicontroller_nm (Utilities|Casting|CastToMyAIControllerNM (Pawn|GetController)))
  (Variables|Default|SetAIController _asmy_aicontroller_nm))

(event Collision|EventActorBeginOverlap
  (params (OtherActor :type Actor%20Object%20Reference)))

(event EventTick
  (params (DeltaSeconds :type Float%20%28single-precision%29)))

(event EventDie
  (if (Utilities|Enum|Equal(Enum) (Networking|GetLocalRole) "ROLE_Authority")
    (Components|Movement|StopMovementImmediately (Variables|Character|GetCharacterMovement))
    (Components|Animation|SetAnimationMode (Variables|Character|GetMesh) "AnimationSingleNode")
    (Components|Animation|SetAnimation (Variables|Character|GetMesh) 0)
    (Actor|DestroyActor)))

(event EventAttack
  (Components|Movement|StopMovementImmediately (Variables|Character|GetCharacterMovement))
  (Components|Animation|SetAnimationMode (Variables|Character|GetMesh) "AnimationSingleNode")
  (Components|Animation|SetAnimation (Variables|Character|GetMesh) 0)
  (Utilities|FlowControl|Delay 2.633)
  (Components|Animation|SetAnimationMode (Variables|Character|GetMesh) "AnimationBlueprint"))

(fn ConstructionScript)