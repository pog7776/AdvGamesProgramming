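; Procedurally generated building that sizes a cube mesh from width, depth and height, either as set or randomized.
; BeginPlay and every Tick check one-shot flags: ApplyValue applies current dimensions, otherwise RandomApplyValue rolls new ones within min/max ranges, then applies them.
; ApplyScale multiplies the dimensions by ScaleFactor, tied to the texture, as the cube's world scale.
; Comments note that the dimension variables live in C++ and a city generator can also randomize buildings.
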(event EventBeginPlay
  ;[1 1 1] for initial execution
  (if (Variables|Control|GetbApplyValue)
    (Variables|Control|SetbApplyValue false)
    (CallFunction|ApplyScale :!label _label)
    (else
      ;[1 1 1] even though city can generate city with random number, single building can be randomly generated as well
      (if (Variables|Control|GetbRandomApplyValue)
        (Variables|Control|SetbRandomApplyValue false)
        (CallFunction|RandomAssignScale)
        (goto _label)))))

(event Collision|EventActorBeginOverlap
  (params (OtherActor :type Actor%20Object%20Reference)))

(event EventTick
  (params (DeltaSeconds :type Float%20%28single-precision%29))
  (if (Variables|Control|GetbApplyValue)
    (Variables|Control|SetbApplyValue false)
    (CallFunction|ApplyScale :!label _label)
    (else
      ;[1 1 1] even though city can generate city with random number, single building can be randomly generated as well
      (if (Variables|Control|GetbRandomApplyValue)
        (Variables|Control|SetbRandomApplyValue false)
        (CallFunction|RandomAssignScale)
        (goto _label)))))

(fn ConstructionScript)

(fn ApplyScale
  (bind _scalefactor (Variables|Default|GetScaleFactor))
  (Transformation|SetWorldScale3D (Variables|Default|GetSimpleCube) (Math|Vector|MakeVector (* _scalefactor (Math|Conversions|ToFloat(Integer) (Variables|Dimension|Getwidth))) (* _scalefactor (Math|Conversions|ToFloat(Integer) (Variables|Dimension|Getdepth))) (* _scalefactor (Math|Conversions|ToFloat(Integer) (Variables|Dimension|Getheight))))))

(fn RandomAssignScale
  (Variables|Dimension|Setwidth (Math|Random|RandomIntegerinRange (Variables|Random|GetminWidth) (Variables|Random|GetmaxWidth)))
  (Variables|Dimension|Setdepth (Math|Random|RandomIntegerinRange (Variables|Random|GetminDepth) (Variables|Random|GetmaxDepth)))
  (Variables|Dimension|Setheight (Math|Random|RandomIntegerinRange (Variables|Random|GetminHeight) (Variables|Random|GetmaxHeight))))