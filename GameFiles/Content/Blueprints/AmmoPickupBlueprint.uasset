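; Ammo pickup actor that refills the reserve ammo of the player's gun when the player character overlaps it.
; It reaches the GunBlueprint through the player's Gun child actor, adds AmmoValue capped at MaxAmmoReserve, then destroys itself.
; A pickup touched at full reserve stays in the world.
; A HUD ammo-text update is present but disconnected, so the pickup does not refresh the display.
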(event EventBeginPlay)

(event Collision|EventActorBeginOverlap
  (params (OtherActor :type Actor%20Object%20Reference))
  (bind _asplayer_character_blueprint (Utilities|Casting|CastToPlayerCharacterBlueprint OtherActor))
  (bind _asgun_blueprint (Utilities|Casting|CastToGunBlueprint (Variables|/Script/Engine.ChildActorComponent|GetChildActor (Variables|/Game/Blueprints/PlayerCharacterBlueprint.PlayerCharacterBlueprint_C|GetGun _asplayer_character_blueprint))))
  (if (not (== (Variables|/Game/Blueprints/GunBlueprint.GunBlueprint_C|GetAmmoReserve _asgun_blueprint) (Variables|/Game/Blueprints/GunBlueprint.GunBlueprint_C|GetMaxAmmoReserve _asgun_blueprint)))
    (if (> (+ (Variables|Default|GetAmmoValue) (Variables|/Game/Blueprints/GunBlueprint.GunBlueprint_C|GetAmmoReserve _asgun_blueprint)) (Variables|/Game/Blueprints/GunBlueprint.GunBlueprint_C|GetMaxAmmoReserve _asgun_blueprint))
      ;[1 1 1] Need to change this to carried ammo
      (Variables|/Game/Blueprints/GunBlueprint.GunBlueprint_C|SetAmmoReserve _asgun_blueprint (Variables|/Game/Blueprints/GunBlueprint.GunBlueprint_C|GetMaxAmmoReserve _asgun_blueprint))
      (else
        (Variables|/Game/Blueprints/GunBlueprint.GunBlueprint_C|SetAmmoReserve _asgun_blueprint (+ (Variables|Default|GetAmmoValue) (Variables|/Game/Blueprints/GunBlueprint.GunBlueprint_C|GetAmmoReserve _asgun_blueprint)))))
    (Actor|DestroyActor)))

(event EventTick
  (params (DeltaSeconds :type Float%20%28single-precision%29)))

(fn ConstructionScript)