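; Weapon pickup Blueprint that transfers its weapon stats to the player's gun when picked up.
; On BeginPlay it calls OnGenerate, then sets the skeletal mesh material to gold, purple, blue or white by rarity tier.
; OnPickup casts to the player character and its Gun child actor, overwrites damage, muzzle velocity, accuracy and magazine size, refills the magazine, then destroys the pickup.
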(event EventBeginPlay
  (bind _skeletalmesh (Variables|Default|GetSkeletalMesh))
  (Class|WeaponPickup|OnGenerate)
  (if (Utilities|Enum|Equal(Enum) (Variables|Default|GetRarity) "LEGENDARY")
    (Rendering|Material|SetMaterial _skeletalmesh 0 "/Game/Materials/Gold.Gold")
    (elif (Utilities|Enum|Equal(Enum) (Variables|Default|GetRarity) "MASTER")
      (Rendering|Material|SetMaterial _skeletalmesh 0 "/Game/Materials/Purple.Purple")
      (elif (Utilities|Enum|Equal(Enum) (Variables|Default|GetRarity) "RARE")
        (Rendering|Material|SetMaterial _skeletalmesh 0 "/Game/Materials/Blue.Blue")
        (elif (Utilities|Enum|Equal(Enum) (Variables|Default|GetRarity) "COMMON")
          (Rendering|Material|SetMaterial _skeletalmesh 0 "/Game/Materials/White.White"))))))

(event Collision|EventActorBeginOverlap
  (params (OtherActor :type Actor%20Object%20Reference)))

(event EventTick
  (params (DeltaSeconds :type Float%20%28single-precision%29)))

(event EventOnPickup
  (params (ActorThatPickedUp :type Actor%20Object%20Reference))
  (bind _asplayer_character_blueprint (Utilities|Casting|CastToPlayerCharacterBlueprint ActorThatPickedUp))
  (bind _asgun_blueprint (Utilities|Casting|CastToGunBlueprint (Variables|/Script/Engine.ChildActorComponent|GetChildActor (Variables|/Game/Blueprints/PlayerCharacterBlueprint.PlayerCharacterBlueprint_C|GetGun _asplayer_character_blueprint))))
  (Variables|/Game/Blueprints/GunBlueprint.GunBlueprint_C|SetBulletDamage _asgun_blueprint (Variables|Default|GetBulletDamage))
  (Variables|/Game/Blueprints/GunBlueprint.GunBlueprint_C|SetMuzzleVelocity _asgun_blueprint (Variables|Default|GetMuzzleVelocity))
  (Variables|/Game/Blueprints/GunBlueprint.GunBlueprint_C|SetWeaponAccuracy _asgun_blueprint (Variables|Default|GetWeaponAccuracy))
  (Variables|/Game/Blueprints/GunBlueprint.GunBlueprint_C|SetMagazineSize _asgun_blueprint (Variables|Default|GetMagazineSize))
  (Variables|/Game/Blueprints/GunBlueprint.GunBlueprint_C|SetRoundsRemainingInMagazine _asgun_blueprint (Variables|Default|GetMagazineSize))
  (Actor|DestroyActor))

(fn ConstructionScript)