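; Gun actor that handles fire-rate cooldown, magazine rounds, instant reload and damage.
; Fire traces a predicted projectile path with random spread instead of spawning a bullet, plays sound and the parent player's arms montage, then damages any HealthComponent hit.
; Hit skeletal meshes get a splatter emitter whose particle collisions spawn temporary decals with random frame and size.
; Tick re-arms firing while rounds remain; debug path drawing and health prints are active.
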(event Custom|On%20Collision
  (params (EventName :type Name) (EmitterTime :type Float%20%28single-precision%29) (ParticleTime :type Integer) (Location :type Vector) (Velocity :type Vector) (Direction :type Vector) (Normal :type Vector) (BoneName :type Name) (PhysMat :type Physical%20Material%20Object%20Reference))
  (bind _returnvalue (Math|Random|RandomFloatinRange 2e+01 5e+01))
  (bind _returnvalue_2 (Math|Conversions|ToVector(Float) _returnvalue))
  (bind (_x _y _z) (Math|Vector|BreakVector _returnvalue_2))
  (bind _returnvalue_3 (Rendering|Material|CreateDynamicMaterialInstance "/Game/Textures/BloodSplatter/Splatters_Decal_M.Splatters_Decal_M" "None" :!class /Script/Engine.KismetMaterialLibrary))
  (Rendering|Material|SetScalarParameterValue _returnvalue_3 "Frame" (Math|Conversions|ToFloat(Integer) (Math|Random|RandomInteger 11)) :!class /Script/Engine.MaterialInstanceDynamic)
  (Rendering|Decal|SpawnDecalatLocation _returnvalue_3 (Math|Vector|MakeVector 1.0 _y _z) Location (Math|Conversions|RotationFromXVector Normal) 2e+01))

(event Custom|On%20Hit%20Actor%20with%20HealthComp
  (params (TargetMesh :type Skeletal%20Mesh%20Component%20Object%20Reference))
  (bind _returnvalue (Effects|SpawnEmitterAttached "/Game/Textures/BloodSplatter/Splatters_P.Splatters_P" TargetMesh "None" "0, 0,150.000000"))
  (EventDispatchers|BindEventtoOnParticleCollide _returnvalue (delegate Custom|On%20Collision)))

(event EventBeginPlay
  (Variables|Default|SetRoundsRemainingInMagazine (Variables|Default|GetMagazineSize)))

(event Collision|EventActorBeginOverlap
  (params (OtherActor :type Actor%20Object%20Reference)))

(event EventTick
  (params (DeltaSeconds :type Float%20%28single-precision%29))
  (if (not (Variables|Default|GetbCanFire))
    (bind _output_get (Variables|Default|SetTimeTillNextShot (- (Variables|Default|GetTimeTillNextShot) DeltaSeconds)))
    (if (and (<= _output_get 0.0) (> (Variables|Default|GetRoundsRemainingInMagazine) 0))
      (Variables|Default|SetbCanFire true))))

(fn ConstructionScript)

(fn Fire
  (params (LaunchDirection :type Vector))
  (bind _muzzleposition (Variables|Default|GetMuzzlePosition))
  (bind _returnvalue (Transformation|GetWorldLocation _muzzleposition))
  (if (Variables|Default|GetbCanFire)
    (Variables|Default|SetbCanFire false)
    (Variables|Default|SetTimeTillNextShot (Variables|Default|GetFireRate))
    (Variables|Default|SetRoundsRemainingInMagazine (- (Variables|Default|GetRoundsRemainingInMagazine) 1))
    (bind _outhit (Class|GameplayStatics|BlueprintPredictProjectilePathbyTraceChannel _returnvalue (* (+ LaunchDirection (/ (Math|Random|RandomUnitVector) (Variables|Default|GetWeaponAccuracy))) (Variables|Default|GetMuzzleVelocity)) true 1.0 "ECC_WorldDynamic" false 0 "ForDuration" 4.0))
    (Audio|PlaySoundatLocation "/Game/Assets/Audio/FirstPersonTemplateWeaponFire02.FirstPersonTemplateWeaponFire02" _returnvalue "0, 0, 0" 1.0 1.0 0.0 0 0 0)
    (bind _asplayer_character_blueprint (Utilities|Casting|CastToPlayerCharacterBlueprint (Actor|GetParentActor))
      (:then
        (Animation|Montage|MontagePlay (Components|SkeletalMesh|GetAnimInstance (Variables|/Game/Blueprints/PlayerCharacterBlueprint.PlayerCharacterBlueprint_C|GetArms _asplayer_character_blueprint)) "/Game/Assets/Arms/Animations/FirstPersonFire_Montage.FirstPersonFire_Montage" 1.0 "MontageLength" 0.0 true))
      (:CastFailed
        _))
    ;[1 1 1] If Hit Actor is not null
    (Utilities|IsValid (.HitActor (Collision|BreakHitResult _outhit))
      (:Is%20Valid
        ;[1 1 1] If Hit Actor's Health Component { is / is not } null
        (Utilities|IsValid (Actor|GetComponentbyClass (.HitActor (Collision|BreakHitResult _outhit)) "/Script/AdvGamesProgramming.HealthComponent")
          (:Is%20Valid
            ;[1 1 1] If Hit Actor's Skeletal Mesh { is / is not } null
            (Utilities|IsValid (Actor|GetComponentbyClass (.HitActor (Collision|BreakHitResult _outhit)) "/Script/Engine.SkeletalMeshComponent")
              (:Is%20Valid
                (CallFunction|OnHitActorwithHealthComp (Actor|GetComponentbyClass (.HitActor (Collision|BreakHitResult _outhit)) "/Script/Engine.SkeletalMeshComponent")))
              (:Is%20Not%20Valid
                _))
            ;[1 1 1] Take Damage anyhow since the target's Health Component is valid
            (Class|HealthComponent|OnTakeDamage (Actor|GetComponentbyClass (.HitActor (Collision|BreakHitResult _outhit)) "/Script/AdvGamesProgramming.HealthComponent") (Variables|Default|GetBulletDamage))
            (Development|PrintString (Utilities|String|ToString(Float) (Variables|/Script/AdvGamesProgramming.HealthComponent|GetCurrentHealth (Actor|GetComponentbyClass (.HitActor (Collision|BreakHitResult _outhit)) "/Script/AdvGamesProgramming.HealthComponent"))) true false))
          (:Is%20Not%20Valid
            (Development|PrintString "Did not hit actor with health component" true false)))))))

(fn Reload
  (Variables|Default|SetRoundsRemainingInMagazine (Variables|Default|GetMagazineSize)))